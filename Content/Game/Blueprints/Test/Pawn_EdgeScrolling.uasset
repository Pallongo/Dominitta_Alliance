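; Test camera pawn with axis-driven movement, edge-scroll offsets and mouse-wheel zoom, starting at a fixed position and rotation.
; Movement follows the camera's forward and right vectors, adding edge axis values that this graph only reads; both handlers are bound to MoveForward.
; Zoom clamps the camera radius, then repositions the camera on a sphere around the pawn using spherical coordinates.
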(event EventBeginPlay
  (Transformation|SetActorLocation "0.000000,0.000000,300.000000" false false)
  (Transformation|SetActorRotation "-90.000000, 0, 0"))

(event Collision|EventActorBeginOverlap
  (params (OtherActor :type Actor%20Object%20Reference)))

(event EventTick
  (params (DeltaSeconds :type Float%20%28single-precision%29)))

(event Input|ActionEvents|InputActionWheelMouseUp
  (params (Key :type Key%20Structure))
  ;[1 1 1] Zoom
  (:Pressed
    (Variables|Default|SetCameraRadius (Math|Float|Clamp(Float) (- (Variables|Default|GetCameraRadius) (Variables|Default|GetZoomSpeed)) (Variables|Default|GetRadiusMin) (Variables|Default|GetRadiusMax)))
    (CallFunction|UpdateCameraLocation)))

(event Input|ActionEvents|InputActionWheelMouseDown
  (params (Key :type Key%20Structure))
  ;[1 1 1] Zoom
  (:Pressed
    (Variables|Default|SetCameraRadius (Math|Float|Clamp(Float) (+ (Variables|Default|GetCameraRadius) (Variables|Default|GetZoomSpeed)) (Variables|Default|GetRadiusMin) (Variables|Default|GetRadiusMax)))
    (CallFunction|UpdateCameraLocation)))

(event Input|AxisEvents|InputAxisMoveForward
  (params (AxisValue :type Float%20%28single-precision%29))
  ;[1 1 1] Movement
  (Transformation|SetActorLocation (Utilities|AddVectortoLocation (Math|Vector|GetForwardVector (Transformation|GetWorldRotation (Variables|Default|GetCameraC))) (* (+ AxisValue (Variables|Default|GetEdgeForwardAxis)) (Variables|Default|GetMovementSpeed))) false false))

(event Input|AxisEvents|InputAxisMoveForward
  (params (AxisValue :type Float%20%28single-precision%29))
  ;[1 1 1] Movement
  (Transformation|SetActorLocation (Utilities|AddVectortoLocation (Math|Vector|GetRightVector (Transformation|GetWorldRotation (Variables|Default|GetCameraC))) (* (+ AxisValue (Variables|Default|GetEdgeRightAxis)) (Variables|Default|GetMovementSpeed))) false false))

(fn ConstructionScript)

(fn UpdateCameraLocation
  (Transformation|SetRelativeLocation (Variables|Default|GetCameraC) (.Location (Utilities|PointonASphere (Variables|Default|GetCameraRadius) (Variables|Default|GetCameraZAngle) (Variables|Default|GetCameraHeightAngle))) false false))