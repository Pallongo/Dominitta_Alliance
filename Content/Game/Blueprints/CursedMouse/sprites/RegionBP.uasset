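; RegionBP is a clickable region sprite, labelled with its region name, that toggles between selected and unselected.
; On BeginPlay it writes RegionName into the RegionText component.
; Clicking the RegionNormal sprite flips IsSelected, tints the sprite blue when selected or restores white when deselected, and plays a menu click sound.
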(event OnClicked(RegionNormal)
  (params (TouchedComponent :type Primitive%20Component%20Object%20Reference) (ButtonPressed :type Key%20Structure))
  (if (Variables|Default|GetisSelected)
    (Sprite|SetSpriteColor (Variables|Default|GetRegionNormal) "(R=1.000000,G=1.000000,B=1.000000,A=5.000000)")
    (Variables|Default|SetisSelected false)
    (Audio|PlaySound2D "/Game/Game/Blueprints/CursedMouse/Sounds/Menu_Selection_Click_1_.Menu_Selection_Click_1_" 1.0 1.0 0.0 0 0)
    (else
      (Sprite|SetSpriteColor (Variables|Default|GetRegionNormal) "(R=0.567708,G=0.578257,B=1.000000,A=5.000000)")
      (Variables|Default|SetisSelected true)
      (Audio|PlaySound2D "/Game/Game/Blueprints/CursedMouse/Sounds/Menu_Selection_Click_1_.Menu_Selection_Click_1_" 1.0 1.0 0.0 0 0))))

(event Collision|EventActorBeginOverlap
  (params (OtherActor :type Actor%20Object%20Reference)))

(event EventTick
  (params (DeltaSeconds :type Float%20%28single-precision%29)))

(event EventBeginPlay
  (Rendering|Components|TextRender|SetText (Variables|Default|GetregionText) (Variables|Default|GetRegionName)))

(fn ConstructionScript)